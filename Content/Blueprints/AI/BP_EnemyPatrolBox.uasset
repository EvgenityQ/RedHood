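; BP_EnemyPatrolBox is an area trigger that tells a set of patrol actors when a player enters or leaves it.
; On begin overlap with an actor implementing BPI_Player, it sends SetCombatTargetMessage with that actor to every entry in PatrolActors.
; On end overlap it sends the same message with no target, clearing the combat target.
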(event `self.ReceiveActorBeginOverlap`
  (params (OtherActor :type "Actor Object Reference"))
  (if (`KismetSystemLibrary.DoesImplementInterface` OtherActor "/Game/Blueprints/Interfaces/BPI_Player.BPI_Player_C")
    (for _array_element (`self.PatrolActors`)
      (message `/Game/Blueprints/Interfaces/BPI_Enemy.SetCombatTarget` _array_element OtherActor))))

(event `self.ReceiveActorEndOverlap`
  (params (OtherActor :type "Actor Object Reference"))
  (if (`KismetSystemLibrary.DoesImplementInterface` OtherActor "/Game/Blueprints/Interfaces/BPI_Player.BPI_Player_C")
    (for _array_element (`self.PatrolActors`)
      (message `/Game/Blueprints/Interfaces/BPI_Enemy.SetCombatTarget` _array_element null))))

(fn `UserConstructionScript`)