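; Base character Blueprint for PaperZD-animated characters, providing melee attacks, health and hit reactions.
; AttackBoxTrace box-traces between two scene points and calls GetHit on any BP_CharacterBase it finds.
; GetHit lowers clamped health, plays the hit override animation, disables input and spawns particles.
; It also shows a floating damage number widget projected above the character, only when that character has a cached PlayerController.
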(event `self.ReceiveBeginPlay`
  (bind _asplayer_controller (cast `PlayerController` (`self.GetController`)))
  (set `self.Player Controller` _asplayer_controller))

(fn `AttackBoxTrace`
  (bind _outhit (`KismetSystemLibrary.BoxTraceSingleForObjects` (`SceneComponent.K2_GetComponentLocation` (`self.BoxTraceStart`)) (`SceneComponent.K2_GetComponentLocation` (`self.BoxTraceEnd`)) (`self.TraceExtent`) (`self.BoxRotation`) (`self.TraceObjectTypes`)))
  (bind _asbp_character_base (cast `/Game/Blueprints/Characters/BP_CharacterBase` (`.HitActor` (`GameplayStatics.BreakHitResult` _outhit))))
  (`self.GetHit` _asbp_character_base (`self.Damage`)))

(fn `CreateDamageNumber`
  (params (Number :type "Float (double-precision)") (Location :type "Vector Structure"))
  (locals (NumberWidget :type "/Game/Blueprints/UI/WBP_DamageNumber Object Reference"))
  (bind (_location_x _location_y _location_z) (`KismetMathLibrary.BreakVector` (`local.Location`)))
  (bind _numberwidget (`local.NumberWidget`))
  (`self.Player Controller`
    (:`then`
      (`|ExecutionSequence`
        (:`then_0`
          ;[0 0.01029 0.15 0.5] Crate Damage Number Widget
          (bind _returnvalue (`|CreateWidget` "/Game/Blueprints/UI/WBP_DamageNumber.WBP_DamageNumber_C" (`self.Player Controller`)))
          (bind _output_get (set `local.NumberWidget` _returnvalue))
          (`UserWidget.AddToViewport` _output_get 0))
        (:`then_1`
          ;[0 0.002575 0.1458 0.5] Set the Number Value
          (`/Game/Blueprints/UI/WBP_DamageNumber.SetNumber` (`local.NumberWidget`) (`local.Number`) (`self.DamageNumberColorAndOpacity`)))
        (:`then_2`
          ;[0.007562 0.01719 0.08854 0.5] Set Position in Viewport
          (`UserWidget.SetPositionInViewport` (`local.NumberWidget`) (`GameplayStatics.ProjectWorldToScreen` (`self.Player Controller`) (`KismetMathLibrary.MakeVector` _location_x _location_y (+ _location_z 75.0))) true))
        (:`then_3`
          ;[0.003321 0.006854 0.1458 0.5] Play Floating Animation
          (`UserWidget.PlayAnimation` _numberwidget (`/Game/Blueprints/UI/WBP_DamageNumber.FloatAnimation` _numberwidget) 0.0 1 "Forward" 1.0 false))))
    (:`else`)))

(fn `DecrementHealth`
  (params (Damage :type "Float (double-precision)"))
  (set `self.Health` (`KismetMathLibrary.FClamp` (- (`self.Health`) Damage) 0.0 (`self.MaxHealth`))))

(fn `GetHit`
  (params (InDamage :type "Float (double-precision)"))
  (`self.DecrementHealth` InDamage)
  (`self.PlayHitReactAnimation`)
  (`self.SetInputEnabled` false)
  (`self.SpawnHitEffects`)
  (`self.CreateDamageNumber` (`local.InDamage`) (`self.K2_GetActorLocation`)))

(fn `PlayAttackAnim`
  (`PaperZDAnimInstance.K2_PlayAnimationOverride` (`PaperZDAnimationComponent.AnimInstance` (`self.PaperZDAnimation`)) (`self.AttackAnimSequence`) "DefaultSlot" 1.0 0.0))

(fn `PlayHitReactAnimation`
  (`PaperZDAnimInstance.K2_PlayAnimationOverride` (`PaperZDAnimationComponent.AnimInstance` (`self.PaperZDAnimation`)) (`self.HitReactAnimSequence`) "DefaultSlot" 1.0 0.0))

(fn `SetInputEnabled`
  (params (Enabled :type Boolean))
  (`self.Player Controller`
    (:`then`
      (if Enabled
        (`self.EnableInput` (`self.Player Controller`))
        (else
          (`self.DisableInput` (`self.Player Controller`)))))
    (:`else`)))

(fn `SpawnHitEffects`
  (`NiagaraFunctionLibrary.SpawnSystemAtLocation` (`self.HitParticles`) (`self.K2_GetActorLocation`)))

(fn `UserConstructionScript`)